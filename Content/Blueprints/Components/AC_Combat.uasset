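; Combat component that manages its owner's weapons: spawning, switching and firing them.
; BuildWeapons spawns each class in WeaponClasses, attaches it to the player's hands socket and stores it by index in WeaponsMap, showing only the first.
; ChangeWeapon notifies via CallOnChangeWeapon and swaps visibility using the weapon type enum as the map key.
; Firing is delegated to the equipped weapon; reload is an empty stub.
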(fn BuildWeapons
  (params (Player%20Hands :type Skeletal%20Mesh%20Component%20Object%20Reference))
  (bind _weapons_map (Variables|Default|GetWeapons%20Map))
  (bind (_value _returnvalue) (Utilities|Map|Find _weapons_map 0))
  (for (_array_element _array_index) (Variables|Default|GetWeapon%20Classes)
    (LocalVariables|SetKey _array_index)
    (bind _returnvalue_2 (Game|SpawnActorfromClass _array_element (Transformation|GetActorTransform (Components|GetOwner)) "AlwaysSpawn" "MultiplyWithRoot" (Components|GetOwner) 0))
    (Utilities|Map|Add (Variables|Default|GetWeapons%20Map) (LocalVariables|GetKey) _returnvalue_2)
    (Transformation|AttachComponentToComponent _returnvalue_2 Player%20Hands (Variables|Default|GetWeapon%20Socket%20Name) "SnapToTarget" "SnapToTarget" "SnapToTarget" false))
  (bind _values (Utilities|Map|Values (Variables|Default|GetWeapons%20Map)))
  (for _array_element_2 _values
    (Rendering|SetActorHiddenInGame _array_element_2 true))
  (if _returnvalue
    (Rendering|SetActorHiddenInGame _value false)
    (Variables|Default|SetEquipped%20Weapon _value)
    (Variables|Default|SetCurrent%20Weapon%20Type "NewEnumerator0")))

(fn ChangeWeapon
  (params (Weapon%20Type :type E_PlayerWeapons%20Enum :default "NewEnumerator0"))
  (bind _output_get (Variables|Default|SetCurrent%20Weapon%20Type Weapon%20Type))
  (Default|CallOnChangeWeapon _output_get)
  (Rendering|SetActorHiddenInGame (Variables|Default|GetEquipped%20Weapon) true)
  (if (.ReturnValue (Utilities|Map|Find (Variables|Default|GetWeapons%20Map) (Math|Conversions|ToInteger(Byte) (Variables|Default|GetCurrent%20Weapon%20Type))))
    (bind _output_get_2 (Variables|Default|SetEquipped%20Weapon (.Value (Utilities|Map|Find (Variables|Default|GetWeapons%20Map) (Math|Conversions|ToInteger(Byte) (Variables|Default|GetCurrent%20Weapon%20Type))))))
    (Rendering|SetActorHiddenInGame _output_get_2 false)))

(fn FireEquippedWeapon
  (params (Player%20Reference :type BP%20Player%20Character%20Object%20Reference))
  (if (Utilities|IsValid (Variables|Default|GetEquipped%20Weapon))
    (Default|FireWeapon (Variables|Default|GetEquipped%20Weapon) Player%20Reference)))

(fn ReloadEquippedWeapon)