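; Player character Blueprint that handles Enhanced Input movement, look, aiming and sprinting, with weapons delegated to CombatComponent.
; A Default/Aiming/Running state sets max walk speed, and a timeline zooms camera FOV for aiming.
; Aim and sprint check each other's held input, so the latest press wins and releasing it restores the other.
; CombatComponent builds weapons on PlayerArms and reports changes; debug keys switch weapons, while shoot input is still empty.
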(event Custom|On%20Change%20Weapon%20Event%20Listener
  (params (Weapon%20Type :type E_PlayerWeapons%20Enum :default "NewEnumerator0"))
  (Variables|Default|SetIs%20Changing%20Weapon true)
  (Variables|Default|SetCurrent%20Weapon Weapon%20Type))

(event EventBeginPlay
  (|BuildMappingContext)
  (StateControl|SetNewPlayerState "NewEnumerator0")
  (EventDispatchers|BindEventtoOnChangeWeapon (Variables|Default|GetCombat%20Component) (EventDispatchers|CreateEvent :!event Custom|On%20Change%20Weapon%20Event%20Listener))
  (Default|BuildWeapons (Variables|Default|GetCombat%20Component) (Variables|Default|GetPlayer%20Arms)))

(event Input|EnhancedActionEvents|EnhancedInputActionIA_Movement
  (params (ActionValue :type Vector%202D%20Structure) (ElapsedSeconds :type Float%20%28double-precision%29) (TriggeredSeconds :type Float%20%28double-precision%29) (InputAction :type Input%20Action%20Object%20Reference :default "/Game/Blueprints/Inputs/IA_Movement.IA_Movement"))
  (bind (_x _y) (Math|Vector2D|BreakVector2D ActionValue))
  ;[0 1 0.2865] Movement
  (Pawn|Input|AddMovementInput (Transformation|GetActorForwardVector) _x false)
  (Pawn|Input|AddMovementInput (Transformation|GetActorRightVector) _y false))

(event Input|EnhancedActionEvents|EnhancedInputActionIA_Look
  (params (ActionValue :type Vector%202D%20Structure) (ElapsedSeconds :type Float%20%28double-precision%29) (TriggeredSeconds :type Float%20%28double-precision%29) (InputAction :type Input%20Action%20Object%20Reference :default "/Game/Blueprints/Inputs/IA_Look.IA_Look"))
  (bind (_x _y) (Math|Vector2D|BreakVector2D ActionValue))
  ;[0 1 0.2865] Look
  (Pawn|Input|AddControllerYawInput _x)
  (Pawn|Input|AddControllerPitchInput _y))

(event Input|EnhancedActionEvents|EnhancedInputActionIA_Aim
  (params (ActionValue :type Boolean) (ElapsedSeconds :type Float%20%28double-precision%29) (TriggeredSeconds :type Float%20%28double-precision%29) (InputAction :type Input%20Action%20Object%20Reference :default "/Game/Blueprints/Inputs/IA_Aim.IA_Aim"))
  ;[0 1 0.2865] Aim
  (:Started
    (StateControl|SetNewPlayerState "NewEnumerator1")
    (bind _field_of_view (Timeline|Aim%20Zoom%20Timeline Play)
      (:Update
        (Camera|SetFieldOfView (Variables|Default|GetCamera) _field_of_view))))
  (:Canceled
    (if (Input|EnhancedActionValues|GetIA_Sprint) :!label _label
      (StateControl|SetNewPlayerState "NewEnumerator3")
      (Timeline|Aim%20Zoom%20Timeline Reverse)
      (else
        (StateControl|SetNewPlayerState "NewEnumerator0")
        (Timeline|Aim%20Zoom%20Timeline Reverse))))
  (:Completed
    (goto _label)))

(event Input|EnhancedActionEvents|EnhancedInputActionIA_Sprint
  (params (ActionValue :type Boolean) (ElapsedSeconds :type Float%20%28double-precision%29) (TriggeredSeconds :type Float%20%28double-precision%29) (InputAction :type Input%20Action%20Object%20Reference :default "/Game/Blueprints/Inputs/IA_Sprint.IA_Sprint"))
  ;[0 1 0.2865] Sprint
  (:Started
    (StateControl|SetNewPlayerState "NewEnumerator3")
    (if (Input|EnhancedActionValues|GetIA_Aim)
      (Utilities|String|Reverse (Variables|Default|GetAim%20Zoom%20Timeline))))
  (:Canceled
    (if (Input|EnhancedActionValues|GetIA_Aim) :!label _label
      (if (not (StateControl|IsAiming))
        (StateControl|SetNewPlayerState "NewEnumerator1")
        (Components|Timeline|PlayfromStart (Variables|Default|GetAim%20Zoom%20Timeline)))
      (else
        (StateControl|SetNewPlayerState "NewEnumerator0"))))
  (:Completed
    (goto _label)))

(event Input|EnhancedActionEvents|EnhancedInputActionIA_Shoot
  (params (ActionValue :type Boolean) (ElapsedSeconds :type Float%20%28double-precision%29) (TriggeredSeconds :type Float%20%28double-precision%29) (InputAction :type Input%20Action%20Object%20Reference :default "/Game/Blueprints/Inputs/IA_Shoot.IA_Shoot"))
  ;[1 1 1] Shoot
)

(event Input|KeyboardEvents|DebugKey1
  (params (Key :type Key%20Structure :default "None") (ActionValue :type Input%20Action%20Value%20Structure))
  (:Pressed
    (Default|ChangeWeapon (Variables|Default|GetCombat%20Component) "NewEnumerator0")))

(event Input|KeyboardEvents|DebugKey4
  (params (Key :type Key%20Structure :default "None") (ActionValue :type Input%20Action%20Value%20Structure))
  (:Pressed
    (Default|ChangeWeapon (Variables|Default|GetCombat%20Component) "NewEnumerator3")))

(event Input|KeyboardEvents|DebugKey2
  (params (Key :type Key%20Structure :default "None") (ActionValue :type Input%20Action%20Value%20Structure))
  (:Pressed
    (Default|ChangeWeapon (Variables|Default|GetCombat%20Component) "NewEnumerator1")))

(event Input|KeyboardEvents|DebugKey3
  (params (Key :type Key%20Structure :default "None") (ActionValue :type Input%20Action%20Value%20Structure))
  (:Pressed
    (Default|ChangeWeapon (Variables|Default|GetCombat%20Component) "NewEnumerator2")))

(fn ConstructionScript)

(fn SetNewPlayerState
  (params (New%20Player%20State :type E_PlayerState%20Enum :default "NewEnumerator0"))
  (bind _output_get (Variables|StateControl|SetPlayer%20State New%20Player%20State))
  (switch Utilities|FlowControl|Switch|SwitchonE_PlayerState _output_get
    (:NewEnumerator0
      (Variables|/Script/Engine.CharacterMovementComponent|SetMaxWalkSpeed (Variables|Character|GetCharacterMovement) (Variables|PlayerMovement|GetWalk%20Movement%20Speed)))
    (:NewEnumerator1
      (Variables|/Script/Engine.CharacterMovementComponent|SetMaxWalkSpeed (Variables|Character|GetCharacterMovement) (Variables|PlayerMovement|GetAim%20Movement%20Speed)))
    (:NewEnumerator3
      (Variables|/Script/Engine.CharacterMovementComponent|SetMaxWalkSpeed (Variables|Character|GetCharacterMovement) (Variables|PlayerMovement|GetRun%20Movement%20Speed)))))

(fn IsAiming
  (return (Utilities|Enum|Equal(Enum) (Variables|StateControl|GetPlayer%20State) "NewEnumerator1")))